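; BP_Generator is a construction-time generator that places static mesh components along a spline.
; The construction script steps along the spline at DistanceSpline intervals, adding a mesh at each point in local space and rotating it to face the spline tangent.
; Unconnected leftover graphs hold alternative experiments: a straight row, a random mesh pick and placement at spline points.
; The event graph has no active logic.
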(event EventBeginPlay)

(event Collision|EventActorBeginOverlap
  (params (OtherActor :type Actor%20Object%20Reference)))

(event EventTick
  (params (DeltaSeconds :type Float%20%28single-precision%29)))

(fn ConstructionScript
  (bind _spline (Variables|Default|GetSpline))
  (bind _distancespline (Variables|Default|GetDistanceSpline))
  (for _index (range 0 (Math|Float|Truncate (/ (Spline|GetSplineLength _spline) _distancespline)))
    (AddComponent|AddStaticMeshComponent false (Math|Transform|MakeTransform (Spline|GetLocationatDistanceAlongSpline _spline (* _index _distancespline) "Local") (Math|Conversions|RotationFromXVector (Spline|GetTangentatDistanceAlongSpline _spline (* _index _distancespline) "Local")) "1.000000,1.000000,1.000000"))))