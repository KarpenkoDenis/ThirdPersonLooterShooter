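; Destructible actor whose static mesh travels along a spline, then is swapped for a physics-simulated Geometry Collection at the end.
; Construction hides the collection with physics off, and Tick moves the mesh at constant speed, drawing debug spheres along the path.
; At the spline's end the collection takes the mesh's relative location and rotation, the mesh is destroyed and Tick stops.
; An on-hit version of the swap is left unconnected.
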(event OnComponentHit(StaticMesh)
  (params (HitComponent :type Primitive%20Component%20Object%20Reference) (OtherActor :type Actor%20Object%20Reference) (OtherComp :type Primitive%20Component%20Object%20Reference) (NormalImpulse :type Vector :default "0, 0, 0") (Hit :type Hit%20Result%20Structure%20%28by%20ref%29)))

(event EventBeginPlay)

(event Collision|EventActorBeginOverlap
  (params (OtherActor :type Actor%20Object%20Reference)))

(event EventTick
  (params (DeltaSeconds :type Float%20%28single-precision%29))
  (bind _staticmesh (Variables|Default|GetStaticMesh))
  (bind _geometrycollection (Variables|Default|GetGeometryCollection))
  (bind _spline (Variables|Default|GetSpline))
  (bind _returnvalue (Transformation|GetRelativeTransform _staticmesh))
  (bind _output_get (Variables|Default|SetCurrDIstance (+ (Variables|Default|GetCurrDIstance) (* DeltaSeconds 3e+03))))
  (if (>= _output_get (Spline|GetSplineLength _spline))
    ;[0.15 0.15 0.15 0.5] подмена меша на разрушаемый объект
    (Transformation|SetWorldTransform _geometrycollection (Math|Transform|MakeTransform (.location _returnvalue) (.rotation _returnvalue) "1.000000,1.000000,1.000000") false false)
    (Development|SetHiddeninGame _geometrycollection false false)
    (Physics|SetSimulatePhysics _geometrycollection true)
    (Components|DestroyComponent _staticmesh)
    (Actor|Tick|SetActorTickEnabled false)
    (else
      (Transformation|SetWorldLocation (Variables|Default|GetStaticMesh) (Spline|GetLocationatDistanceAlongSpline _spline _output_get "World") false true)
      (Rendering|Debug|DrawDebugSphere (Spline|GetLocationatDistanceAlongSpline _spline _output_get "World") 1e+02 12 "(R=1.000000,G=1.000000,B=1.000000,A=1.000000)" 1e+01))))

(fn ConstructionScript
  (bind _geometrycollection (Variables|Default|GetGeometryCollection))
  (Development|SetHiddeninGame _geometrycollection true false)
  (Physics|SetSimulatePhysics _geometrycollection false))