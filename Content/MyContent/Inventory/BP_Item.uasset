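; BP_Item is a world pickup actor that represents an inventory item described by its Info data.
; The construction script sets the static mesh from Info, and SetInfo, run on BeginPlay, stores the data, loads it into the WBP_Item widget and reapplies the mesh.
; When an actor with a BPAC_InventoryComponent overlaps the sphere, the item adds Info to that inventory and destroys itself.
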(event OnComponentBeginOverlap(Sphere)
  (params (OverlappedComponent :type Primitive%20Component%20Object%20Reference) (OtherActor :type Actor%20Object%20Reference) (OtherComp :type Primitive%20Component%20Object%20Reference) (OtherBodyIndex :type Integer) (bFromSweep :type Boolean) (SweepResult :type Hit%20Result%20Structure%20%28by%20ref%29))
  (bind _returnvalue (Actor|GetComponentbyClass OtherActor "/Game/MyContent/Inventory/BPAC_InventoryComponent.BPAC_InventoryComponent_C"))
  (Utilities|IsValid OtherActor
    (:Is%20Valid
      (Utilities|IsValid _returnvalue
        (:Is%20Valid
          (Default|AddItem _returnvalue (Variables|Default|GetInfo))
          (Actor|DestroyActor))))))

(event EventBeginPlay
  (CallFunction|SetInfo (Variables|Default|GetInfo)))

(event Collision|EventActorBeginOverlap
  (params (OtherActor :type Actor%20Object%20Reference)))

(event EventTick
  (params (DeltaSeconds :type Float%20%28single-precision%29)))

(fn ConstructionScript
  (Components|StaticMesh|SetStaticMesh (Variables|Default|GetStaticMesh) (.Mesh (Utilities|Struct|BreakSTRUCT_ItemInfo (Variables|Default|GetInfo)))))

(fn SetInfo
  (params (InfoItem :type STRUCT%20Item%20Info%20Structure))
  (Variables|Default|SetInfo InfoItem)
  (bind _aswbp_item (Utilities|Casting|CastToWBP_Item (UserInterface|GetWidget (Variables|Default|GetWidget))))
  (Default|LoadInfo _aswbp_item InfoItem)
  (Components|StaticMesh|SetStaticMesh (Variables|Default|GetStaticMesh) (.Mesh (Utilities|Struct|BreakSTRUCT_ItemInfo InfoItem))))