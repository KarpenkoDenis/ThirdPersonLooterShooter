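; BP_TVActor is a TV that shows a render target on its screen while a player is nearby.
; BeginPlay builds a dynamic material from M_Base with RenderTargetRef as its "Text" texture, then immediately overrides it with the AdvancedFlag placeholder.
; Sphere overlaps by actors tagged "Player" switch TVScreen to the render-target material on entry and to AnimSharingBlue on exit, so the idle look differs after the first visit.
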(event OnComponentBeginOverlap(Sphere)
  (params (OverlappedComponent :type Primitive%20Component%20Object%20Reference) (OtherActor :type Actor%20Object%20Reference) (OtherComp :type Primitive%20Component%20Object%20Reference) (OtherBodyIndex :type Integer) (bFromSweep :type Boolean) (SweepResult :type Hit%20Result%20Structure%20%28by%20ref%29))
  (if (Actor|ActorHasTag OtherActor "Player")
    (Rendering|Material|SetMaterial (Variables|Default|GetTVScreen) 0 (Variables|Default|GetScreenMaterial))))

(event OnComponentEndOverlap(Sphere)
  (params (OverlappedComponent :type Primitive%20Component%20Object%20Reference) (OtherActor :type Actor%20Object%20Reference) (OtherComp :type Primitive%20Component%20Object%20Reference) (OtherBodyIndex :type Integer))
  (if (Actor|ActorHasTag OtherActor "Player")
    (Rendering|Material|SetMaterial (Variables|Default|GetTVScreen) 0 "/AnimationSharing/AnimSharingBlue.AnimSharingBlue")))

(event EventBeginPlay
  (bind _returnvalue (Rendering|Material|CreateDynamicMaterialInstance "/Game/MyContent/CameraLogic/M_Base.M_Base" "None" "None" :!class /Script/Engine.KismetMaterialLibrary))
  (Rendering|Material|SetTextureParameterValue _returnvalue "Text" (Variables|Default|GetRenderTargetRef))
  (bind _output_get (Variables|Default|SetScreenMaterial _returnvalue))
  (Rendering|Material|SetMaterial (Variables|Default|GetTVScreen) 0 _output_get)
  (Rendering|Material|SetMaterial (Variables|Default|GetTVScreen) 0 "/Engine/MaterialTemplates/VertexAnimation/AdvancedFlag.AdvancedFlag"))

(event Collision|EventActorBeginOverlap
  (params (OtherActor :type Actor%20Object%20Reference)))

(event EventTick
  (params (DeltaSeconds :type Float%20%28single-precision%29)))

(fn ConstructionScript)