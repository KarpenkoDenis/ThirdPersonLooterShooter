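; BP_SpawnWeapon is a one-shot spawner that scatters random weapon items around its location when play begins.
; A loop driven by WeaponNum picks random rows from DT_WeaponInfo and spawns a BP_WeaponItem for each at a random navmesh-reachable point within SpawnRadius.
; Each item receives its row through SetWeaponInfo, and the spawner destroys itself once the loop finishes.
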(event EventBeginPlay
  (bind _outrownames (DataTable|GetDataTableRowNames "/Game/MyContent/DataTables/DT_WeaponInfo.DT_WeaponInfo"))
  (for _index (range 0 (Variables|Default|GetWeaponNum))
    (bind _returnvalue (Utilities|GetDataTableRow "/Game/MyContent/DataTables/DT_WeaponInfo.DT_WeaponInfo" (.OutItem (Utilities|Array|Random _outrownames)))
      (:then
        (bind _returnvalue_2 (Game|SpawnActorfromClass "/Game/MyContent/BP/Inventory/BP_WeaponItem.BP_WeaponItem_C" (Math|Transform|MakeTransform (.RandomLocation (AI|Navigation|GetRandomReachablePointinRadius (Transformation|GetActorLocation) (Variables|Default|GetSpawnRadius) 0 0))) "Undefined" "MultiplyWithRoot" 0 0))
        (Default|SetWeaponInfo _returnvalue_2 _returnvalue))))
  (Actor|DestroyActor))

(event Collision|EventActorBeginOverlap
  (params (OtherActor :type Actor%20Object%20Reference)))

(event EventTick
  (params (DeltaSeconds :type Float%20%28single-precision%29)))

(fn ConstructionScript)