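; Base enemy Blueprint that carries a random item inventory and flags when it sees the player for its AI.
; On BeginPlay it adds a few random rows from the item info data table to its inventory component.
; PawnSensing sets the SeePlayer Blackboard key when it sees a Player-tagged pawn, and nothing here clears it.
; SpawnItemsFromInventory, not called here, spawns each stored item as a BP_Item at random nearby navigable points.
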(event OnSeePawn(PawnSensing)
  (params (Pawn :type Pawn%20Object%20Reference))
  (if (Actor|ActorHasTag Pawn "Player")
    (AI|Components|Blackboard|SetValueasBool (AI|GetBlackboard (AI|GetAIController self)) (Utilities|Name|MakeLiteralName "SeePlayer") true)))

(event EventBeginPlay
  (CallFunction|FillInventorywithRandomItems))

(event Collision|EventActorBeginOverlap
  (params (OtherActor :type Actor%20Object%20Reference)))

(event EventTick
  (params (DeltaSeconds :type Float%20%28single-precision%29)))

(fn ConstructionScript)

(fn FillInventorywithRandomItems
  (for _index (range 0 (Math|Random|RandomIntegerinRange 1 3))
    (bind _outrownames (DataTable|GetDataTableRowNames "/Game/MyContent/DataTables/DT_ItemsInfo.DT_ItemsInfo"))
    (bind _returnvalue (Utilities|GetDataTableRow "/Game/MyContent/DataTables/DT_ItemsInfo.DT_ItemsInfo" (.OutItem (Utilities|Array|Random _outrownames)))
      (:then
        (Default|AddItem (Variables|Default|GetBPAC_InventoryComponent) _returnvalue)))))

(fn SpawnItemsfromInventory
  (bind _items (Default|GetAllItems (Variables|Default|GetBPAC_InventoryComponent)))
  (for _array_element _items
    (bind _randomlocation (Class|NavigationSystemV1|GetRandomLocationinNavigableRadius (Transformation|GetActorLocation) 4e+02 0 0))
    (bind _returnvalue (Game|SpawnActorfromClass "/Game/MyContent/BP/Inventory/BP_Item.BP_Item_C" (Math|Transform|MakeTransform _randomlocation) "Undefined" "MultiplyWithRoot" 0 0))
    (Default|SetInfo _returnvalue _array_element)))