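; Melee AI character that patrols a looping list of points, kicks targets and ragdolls on death.
; TryKick briefly enables DamageSphere, which damages the first overlapped actor with an ACBP_Health component, then switches off; a timer ends the kick.
; GetNextPatrolPoint returns the current point's location and advances the wrapping index.
; Dead detaches the mesh into physics with an impulse, disables movement and capsule collision, and destroys the actor after a delay.
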(event OnComponentBeginOverlap(DamageSphere)
  (params (OverlappedComponent :type Primitive%20Component%20Object%20Reference) (OtherActor :type Actor%20Object%20Reference) (OtherComp :type Primitive%20Component%20Object%20Reference) (OtherBodyIndex :type Integer) (bFromSweep :type Boolean) (SweepResult :type Hit%20Result%20Structure%20%28by%20ref%29))
  (bind _returnvalue (Actor|GetComponentbyClass OtherActor "/Game/MyContent/BP/Weapon/ACBP_Health.ACBP_Health_C"))
  (Utilities|IsValid _returnvalue
    (:Is%20Valid
      (Collision|SetCollisionEnabled (Variables|Default|GetDamageSphere) "NoCollision")
      (Default|Damage _returnvalue (Variables|Default|GetKickForce)))))

(event Custom|DestroyCompletly
  (Actor|DestroyActor))

(event EventBeginPlay
  (Collision|SetCollisionEnabled (Variables|Default|GetDamageSphere) "NoCollision"))

(event Collision|EventActorBeginOverlap
  (params (OtherActor :type Actor%20Object%20Reference)))

(event EventTick
  (params (DeltaSeconds :type Float%20%28single-precision%29)))

(event EventDead
  (params (Impuls :type Vector :default "0, 0, 0") (BoneName :type Name :default "None"))
  (bind _mesh (Variables|Character|GetMesh))
  (Physics|SetSimulatePhysics _mesh true)
  (Transformation|DetachFromComponent _mesh "KeepRelative" "KeepRelative" "KeepRelative" true)
  (Physics|AddImpulse _mesh Impuls BoneName false)
  (Variables|Default|SetAIControllerClass "/Script/AIModule.AIController")
  (Pawn|Components|CharacterMovement|DisableMovement (Variables|Character|GetCharacterMovement))
  (Collision|SetCollisionEnabled (Variables|Default|GetCapsuleComponent) "NoCollision")
  (Utilities|Time|SetTimerbyEvent (delegate Custom|DestroyCompletly) 3e+01))

(fn ConstructionScript)

(fn TryKick
  (if (not (Variables|Default|GetbKick))
    (Variables|Default|SetbKick true)
    (Utilities|Time|SetTimerbyFunctionName 0 "FinishKick" (Variables|Default|GetKickTime))
    (Collision|SetCollisionEnabled (Variables|Default|GetDamageSphere) "QueryAndPhysics")))

(fn FinishKick
  (Variables|Default|SetbKick false)
  (Development|PrintString "Finish" true true "(R=0.379749,G=1.000000,B=0.000000,A=1.000000)" 0.5 (Utilities|String|StringToName (Utilities|GetObjectName self)))
  (Collision|SetCollisionEnabled (Variables|Default|GetDamageSphere) "NoCollision"))

(fn GetNextPatrolPoint
  (LocalVariables|SetNextPoint (Transformation|GetActorLocation (Utilities|Array|Get(acopy) (Variables|Default|GetPatrolPoints) (Variables|Default|GetLastPointIndex))))
  (bind _result (Math|Integer|IncrementInt (Variables|Default|GetLastPointIndex))
    (:%20%20
      (bind _output_get (Variables|Default|SetLastPointIndex (Math|Integer|%(Integer) _result (Utilities|Array|Length (Variables|Default|GetPatrolPoints)))))
      (Development|PrintString (Utilities|String|ToString(Integer) _output_get))
      (return (LocalVariables|GetNextPoint)))))