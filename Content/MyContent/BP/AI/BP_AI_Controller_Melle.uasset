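; AI controller for the melee enemy BP_Melle that wanders the navmesh, chases the player and kicks at close range.
; On begin play it picks a random navigable point and caches the pawn reference.
; Each tick, unless the pawn is kicking, distance checks choose between picking a new wander point near arrival, moving toward a nearby player, or calling TryKick when very close.
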(event EventBeginPlay
  (CallFunction|MovetoRandomLocation)
  (bind _asbp_melle (Utilities|Casting|CastToBP_Melle (Pawn|GetControlledPawn)))
  (bind _output_get (Variables|Default|SetMellePawnRef _asbp_melle)))

(event EventTick
  (params (DeltaSeconds :type Float%20%28single-precision%29))
  (bind _returnvalue (Game|Player|GetPlayerPawn 0))
  (bind _returnvalue_2 (Pawn|GetControlledPawn))
  (bind _returnvalue_3 (Transformation|GetActorLocation _returnvalue))
  (bind _returnvalue_4 (Transformation|GetActorLocation _returnvalue_2))
  (bind _returnvalue_5 (Math|Vector|Distance(Vector) _returnvalue_3 _returnvalue_4))
  (if (not (Variables|/Game/MyContent/BP/AI/BP_Melle.BP_Melle_C|GetbKick (Variables|Default|GetMellePawnRef)))
    (if (> _returnvalue_5 1e+03)
      (if (< (Math|Vector|Distance(Vector) (Transformation|GetActorLocation (Pawn|GetControlledPawn)) (Variables|Default|GetDest)) 2e+02)
        (CallFunction|MovetoRandomLocation))
      (elif (< _returnvalue_5 1e+02)
        (Default|TryKick (Variables|Default|GetMellePawnRef))
        (else
          (CallFunction|MovetoPlayer))))))

(fn ConstructionScript)

(fn MovetoRandomLocation
  ;[0.15 0.15 0.15 0.5] поиск точки и движение к ней
  (bind _randomlocation (Class|NavigationSystemV1|GetRandomLocationinNavigableRadius (Transformation|GetActorLocation (Pawn|GetControlledPawn)) 1e+04 0 0))
  (bind _output_get (Variables|Default|SetDest _randomlocation))
  (bind _returnvalue (AI|Navigation|MovetoLocation _output_get -1.0 true true true true 0))
  (Development|PrintString (Utilities|String|EnumtoString _returnvalue)))

(fn MovetoPlayer
  (AI|Navigation|MovetoActor (Game|Player|GetPlayerPawn 0) -1.0 true true true 0))