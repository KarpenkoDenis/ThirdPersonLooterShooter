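; Player character Blueprint with Enhanced Input movement, look, stamina-limited sprint, inventory toggle, main HUD and ragdoll death.
; Jump first traces forward for an actor tagged "Crouch"; on a hit, a Timeline moves the character up and over with input disabled.
; Fire traces from the camera to aim the child-actor weapon's shot from its muzzle.
; Debug prints and draws remain, older aiming and damage experiments are disconnected, and Damage always returns false.
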(event Custom|CustomEvent)

(event Input|EnhancedActionEvents|EnhancedInputActionIA_Move
  (params (ActionValue :type Vector%202D%20Structure) (ElapsedSeconds :type Float%20%28double-precision%29) (TriggeredSeconds :type Float%20%28double-precision%29) (InputAction :type Input%20Action%20Object%20Reference :default "/Game/MyContent/Input/IA_Move.IA_Move"))
  (bind _returnvalue (Pawn|GetControlRotation :!class /Script/Engine.Pawn))
  (bind (_x _y) (Math|Vector2D|BreakVector2D ActionValue))
  (Variables|Default|SetMovementVector ActionValue)
  (Pawn|Input|AddMovementInput (Math|Vector|GetRightVector (Math|Rotator|MakeRotator (.roll _returnvalue) 0.0 (.yaw _returnvalue))) _x false)
  (Pawn|Input|AddMovementInput (Math|Vector|GetForwardVector (Math|Rotator|MakeRotator 0.0 0.0 (.yaw (Pawn|GetControlRotation :!class /Script/Engine.Pawn)))) _y false))

(event Input|EnhancedActionEvents|EnhancedInputActionIA_Look
  (params (ActionValue :type Vector%202D%20Structure) (ElapsedSeconds :type Float%20%28double-precision%29) (TriggeredSeconds :type Float%20%28double-precision%29) (InputAction :type Input%20Action%20Object%20Reference :default "/Game/MyContent/Input/IA_Look.IA_Look"))
  (bind (_x _y) (Math|Vector2D|BreakVector2D ActionValue))
  (Pawn|Input|AddControllerYawInput _x)
  (Pawn|Input|AddControllerPitchInput _y)
  (Variables|Default|SetPitch _y)
  (Variables|Default|SetYaw (Math|Float|Clamp(Float) (+ (Variables|Default|GetYaw) _x) -6e+01 6e+01)))

(event Input|EnhancedActionEvents|EnhancedInputActionIA_Jump
  (params (ActionValue :type Boolean) (ElapsedSeconds :type Float%20%28double-precision%29) (TriggeredSeconds :type Float%20%28double-precision%29) (InputAction :type Input%20Action%20Object%20Reference :default "/Game/MyContent/Input/IA_Jump.IA_Jump"))
  (bind _returnvalue (Transformation|GetActorLocation))
  (bind (_result _directiontoobstacle) (CallFunction|Check))
  (:Started
    (if _result
      (Variables|Default|SetDirection%20to%20Obstacle (/ _directiontoobstacle 15))
      (Development|PrintString "Not jump")
      (Variables|Default|SetbClimbing true)
      (Input|DisableInput (Game|GetPlayerController 0))
      (Variables|Default|SetSavedLocation (Transformation|GetActorLocation))
      (bind _newtrack_0 (Timeline|Timeline PlayFromStart)
        (:Update
          (if (> _newtrack_0 0.8)
            (Transformation|SetActorLocation (Math|Vector|MakeVector (+ (.x (Variables|Default|GetDirection%20to%20Obstacle)) (.x _returnvalue)) (+ (.y (Variables|Default|GetDirection%20to%20Obstacle)) (.y _returnvalue)) (+ (.z (Variables|Default|GetSavedLocation)) (* _newtrack_0 (Variables|Default|GetClimbDistance)))) false false)
            (Development|PrintString "end 20")
            (Rendering|Debug|DrawDebugLine (Variables|Default|GetSavedLocation) (Math|Vector|MakeVector (+ (.x (Variables|Default|GetDirection%20to%20Obstacle)) (.x _returnvalue)) (+ (.y (Variables|Default|GetDirection%20to%20Obstacle)) (.y _returnvalue)) (+ (.z (Variables|Default|GetSavedLocation)) (* _newtrack_0 (Variables|Default|GetClimbDistance)))) "(R=0.344547,G=1.000000,B=0.000000,A=1.000000)" 0.0 0.0)
            (else
              (Transformation|SetActorLocation (Math|Vector|MakeVector (.x (Variables|Default|GetSavedLocation)) (.y (Variables|Default|GetSavedLocation)) (+ (.z (Variables|Default|GetSavedLocation)) (* _newtrack_0 (Variables|Default|GetClimbDistance)))) false false)))
          (Rendering|Debug|DrawDebugSphere (Variables|Default|GetSavedLocation) 1e+02 12 "(R=1.000000,G=1.000000,B=1.000000,A=1.000000)" 1e+02))
        (:Finished
          (Variables|Default|SetbClimbing false)
          (Input|EnableInput (Game|GetPlayerController 0))))
      (else
        (Character|Jump)
        (Variables|Default|SetbJumping true))))
  (:Completed
    (Character|StopJumping)
    (Variables|Default|SetbJumping false)))

(event Input|EnhancedActionEvents|EnhancedInputActionIA_Shift
  (params (ActionValue :type Boolean) (ElapsedSeconds :type Float%20%28double-precision%29) (TriggeredSeconds :type Float%20%28double-precision%29) (InputAction :type Input%20Action%20Object%20Reference :default "/Game/MyContent/Input/IA_Shift.IA_Shift"))
  (:Started
    (Variables|/Script/Engine.CharacterMovementComponent|SetMaxWalkSpeed (Variables|Character|GetCharacterMovement) (Variables|Default|GetShiftSpeed))
    (Variables|Default|SetbShifting true))
  (:Completed
    (Variables|/Script/Engine.CharacterMovementComponent|SetMaxWalkSpeed (Variables|Character|GetCharacterMovement) (Variables|Default|GetSpeed))
    (Variables|Default|SetbShifting false)))

(event Input|EnhancedActionEvents|EnhancedInputActionIA_Fire
  (params (ActionValue :type Boolean) (ElapsedSeconds :type Float%20%28double-precision%29) (TriggeredSeconds :type Float%20%28double-precision%29) (InputAction :type Input%20Action%20Object%20Reference :default "/Game/MyContent/Input/IA_Fire.IA_Fire"))
  (bind _weaponref (Variables|Default|GetWeaponRef))
  (bind _weaponref_2 (Variables|Default|GetWeaponRef))
  (bind _camera (Variables|Default|GetCamera))
  (bind _returnvalue (Transformation|GetWorldLocation _camera))
  (bind _bulletloc (Default|GetBulletLocation _weaponref))
  (bind _bcanshoot (Default|CanShoot _weaponref_2))
  (if _bcanshoot
    (Default|MakeFire _weaponref_2)
    ;[0.15 0.15 0.15 0.5] определить положение поверхности под курсором
    (bind (_outhit _returnvalue_2) (Collision|LineTraceByChannel _returnvalue (+ _returnvalue (* (Math|Vector|GetForwardVector (Transformation|GetWorldRotation _camera)) (Variables|/Game/MyContent/BP/Weapon/BP_WeaponBase.BP_WeaponBase_C|GetRange (Variables|Default|GetWeaponRef)))) "TraceTypeQuery1" false 0 "None"))
    (if _returnvalue_2
      ;[0.15 0.15 0.15 0.5] стрельба к поверхности курсора
      (Default|Shot _weaponref _bulletloc (.Location (Collision|BreakHitResult _outhit)))
      (else
        (Default|Shot (Variables|Default|GetWeaponRef) _bulletloc (* (Math|Vector|GetForwardVector (Transformation|GetWorldRotation (Variables|Default|GetCamera))) (Variables|/Game/MyContent/BP/Weapon/BP_WeaponBase.BP_WeaponBase_C|GetRange (Variables|Default|GetWeaponRef))))))))

(event Input|EnhancedActionEvents|EnhancedInputActionIA_OpenInventory
  (params (ActionValue :type Boolean) (ElapsedSeconds :type Float%20%28double-precision%29) (TriggeredSeconds :type Float%20%28double-precision%29) (InputAction :type Input%20Action%20Object%20Reference :default "/Game/MyContent/Input/IA_OpenInventory.IA_OpenInventory"))
  (:Started
    (Default|SwitchInventory (Variables|Default|GetBPAC_InventoryComponent))))

(event EventBeginPlay
  (Utilities|FlowControl|Sequence
    (:then_0
      (Input|AddMappingContext (PlayerController|LocalPlayerSubsystems|GetEnhancedInputLocalPlayerSubsystem (Game|GetPlayerController 0)) "/Game/MyContent/Input/IMC_MappingContexts.IMC_MappingContexts" 0 "(bIgnoreAllPressedKeysUntilRelease=True,bForceImmediately=False,bNotifyUserSettings=False)")
      (bind _asbp_weapon_base (Utilities|Casting|CastToBP_WeaponBase (Variables|/Script/Engine.ChildActorComponent|GetChildActor (Variables|Default|GetWeaponComp)))
        (:then
          (bind _output_get (Variables|Default|SetWeaponRef _asbp_weapon_base)))
        (:CastFailed
          (Development|PrintString "Wrong Weapon" true true "(R=0.000000,G=0.660000,B=1.000000,A=1.000000)" 2e+01))))
    (:then_1
      (bind _returnvalue (UserInterface|CreateWidget "/Game/MyContent/Widgets/WBP_MainHUD.WBP_MainHUD_C"))
      (Variables|Default|SetHUD_Ref _returnvalue)
      (UserInterface|Viewport|AddtoViewport _returnvalue 0))))

(event EventDead
  (params (Impuls :type Vector :default "0, 0, 0") (BoneName :type Name :default "None"))
  (bind _mesh (Variables|Character|GetMesh))
  (Physics|SetSimulatePhysics _mesh true)
  (Collision|SetCollisionProfileName _mesh "BlockAll" true :!class /Script/Engine.PrimitiveComponent)
  (Transformation|DetachFromComponent _mesh "KeepRelative" "KeepRelative" "KeepRelative" true)
  (Physics|AddImpulse _mesh Impuls BoneName false)
  (Pawn|Components|CharacterMovement|DisableMovement (Variables|Character|GetCharacterMovement))
  (Collision|SetCollisionEnabled (Variables|Collision|GetCapsuleComponent) "NoCollision"))

(event EventTick
  (params (DeltaSeconds :type Float%20%28single-precision%29))
  (Utilities|FlowControl|Sequence
    (:then_0
      (if (Variables|Default|GetbShifting)
        (bind _output_get (Variables|Default|SetStamina (- (Variables|Default|GetStamina) DeltaSeconds)))
        (if (<= (Variables|Default|GetStamina) 0.0)
          (Variables|Default|SetbShifting false)
          (Variables|/Script/Engine.CharacterMovementComponent|SetMaxWalkSpeed (Variables|Character|GetCharacterMovement) (Variables|Default|GetSpeed)))
        (elif (<= (Variables|Default|GetStamina) 1e+01)
          (Variables|Default|SetStamina (+ (Variables|Default|GetStamina) DeltaSeconds)))))
    (:then_1)
    (:then_2
      (Development|PrintString (Utilities|String|Append "PlayerHP: " (Utilities|String|ToString(Float) (Variables|/Game/MyContent/BP/Weapon/ACBP_Health.ACBP_Health_C|GetHP (Variables|Default|GetACBP_Health)))) true true "(R=0.000000,G=1.000000,B=0.000000,A=1.000000)" -1.0 "PlayerHP"))))

(event Input|KeyboardEvents|E
  (params (Key :type Key%20Structure :default "None"))
  (:Pressed
    (Variables|Default|SetbGrabItem true)))

(fn ConstructionScript)

(fn Check
  (bind _returnvalue (Transformation|GetActorLocation))
  (bind (_outhit _returnvalue_2) (Collision|LineTraceByChannel _returnvalue (+ _returnvalue (* (Math|Vector|GetForwardVector (Transformation|GetActorRotation)) (Variables|Default|GetClimbDetectTraceDistance))) "TraceTypeQuery1" false 0 "ForDuration"))
  (if _returnvalue_2
    (Utilities|IsValid (.HitActor (Collision|BreakHitResult _outhit))
      (:Is%20Valid
        (return (Actor|ActorHasTag (.HitActor (Collision|BreakHitResult _outhit)) "Crouch") (- (.Location (Collision|BreakHitResult _outhit)) (Transformation|GetActorLocation)))))
    (else
      (return false "0, 0, 0"))))

(fn SetWeaponType
  (params (InClass :type Actor%20Class%20Reference))
  (bind _weaponcomp (Variables|Default|GetWeaponComp))
  (ChildActorComponent|SetChildActorClass _weaponcomp InClass)
  (bind _asbp_weapon_base (Utilities|Casting|CastToBP_WeaponBase (Variables|/Script/Engine.ChildActorComponent|GetChildActor _weaponcomp)))
  (Variables|Default|SetWeaponRef _asbp_weapon_base))

(fn Damage
  (params (Val :type Float%20%28double-precision%29))
  (return false))