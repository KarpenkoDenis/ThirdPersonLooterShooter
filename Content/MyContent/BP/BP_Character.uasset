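; Player character Blueprint with camera-relative movement, look, jump and a stamina-limited sprint.
; BeginPlay adds the Enhanced Input mapping context, and input actions drive movement, controller rotation, jumping and walk-speed switching.
; Tick drains Stamina while sprinting, restores normal speed when it runs out, and otherwise refills it to about a fixed cap.
; Move, look and stamina values print on screen for debugging.
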(event Input|EnhancedActionEvents|EnhancedInputActionIA_Move
  (params (ActionValue :type Vector%202D%20Structure) (ElapsedSeconds :type Float%20%28double-precision%29) (TriggeredSeconds :type Float%20%28double-precision%29) (InputAction :type Input%20Action%20Object%20Reference :default "/Game/MyContent/Input/IA_Move.IA_Move"))
  (bind _returnvalue (Pawn|GetControlRotation :!class /Script/Engine.Pawn))
  (bind (_x _y) (Math|Vector2D|BreakVector2D ActionValue))
  (:Triggered
    (Variables|Default|SetMovementVector ActionValue)
    (Development|PrintString (Utilities|String|ToString(Vector2d) ActionValue) true true "(R=0.000000,G=0.660000,B=1.000000,A=1.000000)" 2.0 "Move")
    (Pawn|Input|AddMovementInput (Math|Vector|GetRightVector (Math|Rotator|MakeRotator (.roll _returnvalue) 0.0 (.yaw _returnvalue))) _x false)
    (Pawn|Input|AddMovementInput (Math|Vector|GetForwardVector (Math|Rotator|MakeRotator 0.0 0.0 (.yaw (Pawn|GetControlRotation :!class /Script/Engine.Pawn)))) _y false)))

(event Input|EnhancedActionEvents|EnhancedInputActionIA_Look
  (params (ActionValue :type Vector%202D%20Structure) (ElapsedSeconds :type Float%20%28double-precision%29) (TriggeredSeconds :type Float%20%28double-precision%29) (InputAction :type Input%20Action%20Object%20Reference :default "/Game/MyContent/Input/IA_Look.IA_Look"))
  (bind (_x _y) (Math|Vector2D|BreakVector2D ActionValue))
  (:Triggered
    (Development|PrintString (Utilities|String|ToString(Vector2d) ActionValue) true true "(R=0.000000,G=0.081684,B=1.000000,A=1.000000)" 2.0 "Look")
    (Pawn|Input|AddControllerYawInput _x)
    (Pawn|Input|AddControllerPitchInput _y)))

(event Input|EnhancedActionEvents|EnhancedInputActionIA_Jump
  (params (ActionValue :type Boolean) (ElapsedSeconds :type Float%20%28double-precision%29) (TriggeredSeconds :type Float%20%28double-precision%29) (InputAction :type Input%20Action%20Object%20Reference :default "/Game/MyContent/Input/IA_Jump.IA_Jump"))
  (:Started
    (Character|Jump)
    (Variables|Default|SetbJumping true))
  (:Completed
    (Character|StopJumping)
    (Variables|Default|SetbJumping false)))

(event Input|EnhancedActionEvents|EnhancedInputActionIA_Shift
  (params (ActionValue :type Boolean) (ElapsedSeconds :type Float%20%28double-precision%29) (TriggeredSeconds :type Float%20%28double-precision%29) (InputAction :type Input%20Action%20Object%20Reference :default "/Game/MyContent/Input/IA_Shift.IA_Shift"))
  (:Started
    (Variables|/Script/Engine.CharacterMovementComponent|SetMaxWalkSpeed (Variables|Character|GetCharacterMovement) (Variables|Default|GetShiftSpeed))
    (Variables|Default|SetbShifting true))
  (:Completed
    (Variables|/Script/Engine.CharacterMovementComponent|SetMaxWalkSpeed (Variables|Character|GetCharacterMovement) (Variables|Default|GetSpeed))
    (Variables|Default|SetbShifting false)))

(event EventBeginPlay
  (Input|AddMappingContext (PlayerController|LocalPlayerSubsystems|GetEnhancedInputLocalPlayerSubsystem (Game|GetPlayerController 0)) "/Game/MyContent/Input/IMC_MappingContexts.IMC_MappingContexts" 0 "(bIgnoreAllPressedKeysUntilRelease=True,bForceImmediately=False,bNotifyUserSettings=False)"))

(event Collision|EventActorBeginOverlap
  (params (OtherActor :type Actor%20Object%20Reference)))

(event EventTick
  (params (DeltaSeconds :type Float%20%28single-precision%29))
  (if (Variables|Default|GetbShifting)
    (bind _output_get (Variables|Default|SetStamina (- (Variables|Default|GetStamina) DeltaSeconds)))
    (Development|PrintString (Utilities|String|ToString(Float) _output_get) true true "(R=0.000000,G=0.660000,B=1.000000,A=1.000000)" 2.0 "Stamina")
    (if (<= (Variables|Default|GetStamina) 0.0)
      (Variables|Default|SetbShifting false)
      (Variables|/Script/Engine.CharacterMovementComponent|SetMaxWalkSpeed (Variables|Character|GetCharacterMovement) (Variables|Default|GetSpeed)))
    (elif (<= (Variables|Default|GetStamina) 1e+01)
      (Variables|Default|SetStamina (+ (Variables|Default|GetStamina) DeltaSeconds)))))

(fn ConstructionScript)