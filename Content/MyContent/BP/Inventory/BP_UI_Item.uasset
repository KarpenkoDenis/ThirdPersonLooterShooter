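; BP_UI_Item is an inventory item actor that the player rotates by clicking and dragging the mouse on its Sphere component.
; A click stores the viewport mouse position and sets Active; release clears it.
; While Active, Tick maps the drag offset from that start point directly to absolute roll and pitch, ignoring prior rotation.
; The forward vector saved on click is unused here, and debug prints remain.
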(event OnClicked(Sphere)
  (params (TouchedComponent :type Primitive%20Component%20Object%20Reference) (ButtonPressed :type Key%20Structure :default "None"))
  (Variables|Default|SetbActive true)
  (Development|PrintString "Mouse click")
  (Variables|Default|SetSaveDirection (Transformation|GetActorForwardVector))
  (bind _returnvalue (Class|WidgetLayoutLibrary|GetMousePositiononViewport))
  (Variables|Default|SetStartMousePosition _returnvalue))

(event OnReleased(Sphere)
  (params (TouchedComponent :type Primitive%20Component%20Object%20Reference) (ButtonReleased :type Key%20Structure :default "None"))
  (Variables|Default|SetbActive false)
  (Development|PrintString "Mouse release"))

(event EventBeginPlay)

(event Collision|EventActorBeginOverlap
  (params (OtherActor :type Actor%20Object%20Reference)))

(event EventTick
  (params (DeltaSeconds :type Float%20%28single-precision%29))
  (if (Variables|Default|GetbActive)
    (Development|PrintString "tick")
    (bind _returnvalue (Class|WidgetLayoutLibrary|GetMousePositiononViewport))
    (Development|PrintString (Utilities|String|ToString(Vector2d) (- (Variables|Default|GetStartMousePosition) _returnvalue)))
    (Transformation|SetActorRotation (Math|Rotator|MakeRotator (.x (Class|KismetMathLibrary|GetRotated2D (- (Variables|Default|GetStartMousePosition) _returnvalue) 0.0)) (.y (Class|KismetMathLibrary|GetRotated2D (- (Variables|Default|GetStartMousePosition) _returnvalue) 0.0)) 0.0))))

(fn ConstructionScript)