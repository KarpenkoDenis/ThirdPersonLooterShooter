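; BP_WeaponItem is a weapon pickup item that extends a parent item Blueprint with a weapon type.
; On sphere overlap, it adds its Info to the overlapping actor's BPAC_InventoryComponent, then sets the weapon type if that actor is BP_PlayerCharacter.
; SetWeaponInfo passes Info to the parent's SetInfo and stores the WeaponType.
; The overlap logic does not destroy or hide the item.
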(event OnComponentBeginOverlap(Sphere)
  (params (OverlappedComponent :type Primitive%20Component%20Object%20Reference) (OtherActor :type Actor%20Object%20Reference) (OtherComp :type Primitive%20Component%20Object%20Reference) (OtherBodyIndex :type Integer) (bFromSweep :type Boolean) (SweepResult :type Hit%20Result%20Structure%20%28by%20ref%29))
  (bind _returnvalue (Actor|GetComponentbyClass OtherActor "/Game/MyContent/BP/Inventory/BPAC_InventoryComponent.BPAC_InventoryComponent_C"))
  (Utilities|IsValid OtherActor
    (:Is%20Valid
      (Utilities|IsValid _returnvalue
        (:Is%20Valid
          (Default|AddItem _returnvalue (Variables|Default|GetInfo))
          (bind _asbp_player_character (Utilities|Casting|CastToBP_PlayerCharacter OtherActor))
          (Default|SetWeaponType _asbp_player_character (Variables|Default|GetWeaponType)))))))

(event EventBeginPlay
  (|CallParentFunction) ; This node is disabled and will not be called.\nDrag off pins to build functionality.
)

(event Collision|EventActorBeginOverlap
  (params (OtherActor :type Actor%20Object%20Reference))
  (|CallParentFunction OtherActor) ; This node is disabled and will not be called.\nDrag off pins to build functionality.
)

(event EventTick
  (params (DeltaSeconds :type Float%20%28single-precision%29))
  (|CallParentFunction DeltaSeconds) ; This node is disabled and will not be called.\nDrag off pins to build functionality.
)

(fn ConstructionScript
  (|CallParentFunction))

(fn SetWeaponInfo
  (params (Info :type STRUCT%20Item%20Info%20Structure) (WeaponType :type BP%20Weapon%20Base%20Class%20Reference))
  (|CallParentFunction Info)
  (Variables|Default|SetWeaponType WeaponType))