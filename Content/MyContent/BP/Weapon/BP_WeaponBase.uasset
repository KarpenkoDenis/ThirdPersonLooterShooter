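; BP_WeaponBase is a weapon Blueprint providing fire-rate gating, hit damage and a bullet origin.
; MakeFire sets the firing flag and blocks shooting until a timer, derived from FireRate, calls ChangeCanShoot.
; MakeDamage sends Damage through the target's DamageMessage, spawns an impact emitter, and on a true result adds another emitter and destroys the target.
; GetBulletLocation returns the Arrow component's position; tracing and input are absent here.
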(event EventBeginPlay)

(event Collision|EventActorBeginOverlap
  (params (OtherActor :type Actor%20Object%20Reference)))

(event EventTick
  (params (DeltaSeconds :type Float%20%28single-precision%29)))

(fn ConstructionScript)

(fn MakeFire
  (Variables|Default|SetbFire true)
  (Variables|Default|SetbCanShoot false)
  (Utilities|Time|SetTimerbyFunctionName 0 "ChangeCanShoot" (/ 1.0 (Variables|Default|GetFireRate))))

(fn ChangeCanShoot
  (Variables|Default|SetbCanShoot true)
  (Variables|Default|SetbFire false))

(fn CanShoot
  (return (Variables|Default|GetbCanShoot)))

(fn MakeDamage
  (params (TargetActor :type Actor%20Object%20Reference) (HitLocation :type Vector))
  (bind _bdead (Class|BPIDamageble|Damage(Message) TargetActor (Variables|Default|GetDamage)))
  (Effects|SpawnEmitteratLocation "/Engine/Tutorial/SubEditors/TutorialAssets/TutorialParticleSystem.TutorialParticleSystem" HitLocation "0, 0, 0" "0.300000,0.300000,0.300000")
  (if _bdead
    (Effects|SpawnEmitteratLocation (Variables|Default|GetEmitter%20Template) (Transformation|GetActorLocation TargetActor))
    (Actor|DestroyActor TargetActor)))

(fn GetBulletLocation
  (return (Transformation|GetWorldLocation (Variables|Default|GetArrow))))