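; BP_Bullet is a projectile actor that damages actors with an ACBP_Health component and destroys itself on such a hit.
; Its DamageCollision overlap skips Player-tagged actors unless EnemyBullet is set; other actors can be hit by either bullet type.
; Hits pass damage power, a velocity-scaled impulse and the hit bone to DamageWithImpuls.
; SetBulletType stores the enemy flag and applies a red material to the sphere whatever its value.
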(event OnComponentBeginOverlap(DamageCollision)
  (params (OverlappedComponent :type Primitive%20Component%20Object%20Reference) (OtherActor :type Actor%20Object%20Reference) (OtherComp :type Primitive%20Component%20Object%20Reference) (OtherBodyIndex :type Integer) (bFromSweep :type Boolean) (SweepResult :type Hit%20Result%20Structure%20%28by%20ref%29))
  (bind _returnvalue (Actor|ActorHasTag OtherActor "Player"))
  (bind _returnvalue_2 (Actor|GetComponentbyClass OtherActor "/Game/MyContent/BP/Weapon/ACBP_Health.ACBP_Health_C"))
  (if (or (and _returnvalue (Variables|Default|GetbEnemyBullet)) (not _returnvalue))
    (Utilities|IsValid _returnvalue_2
      (:Is%20Valid
        (Default|DamagewithImpuls _returnvalue_2 (Variables|Default|GetDamagePower) (* (Transformation|GetVelocity) 1e+02) (.BoneName (Collision|BreakHitResult SweepResult)))
        (Actor|DestroyActor)))))

(event EventBeginPlay)

(event Collision|EventActorBeginOverlap
  (params (OtherActor :type Actor%20Object%20Reference)))

(event EventTick
  (params (DeltaSeconds :type Float%20%28single-precision%29)))

(fn ConstructionScript)

(fn SetBulletType
  (params (bEnemyBullet :type Boolean))
  (Variables|Default|SetbEnemyBullet bEnemyBullet)
  (Rendering|Material|SetMaterial (Variables|Default|GetSphere) 0 "/AnimationSharing/AnimSharingRed.AnimSharingRed"))