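; BP_Rifle is a rifle weapon Blueprint that configures its stats from data when play begins.
; After the parent BeginPlay, it reads the "Rifle" row of DT_WeaponSettings to set max ammo and fire rate, and fills current ammo to the maximum.
; It adds no firing logic of its own; leftover unconnected nodes for printing a random table row and spawning BP_WeaponBase never run.
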(event EventBeginPlay
  (|CallParentFunction)
  (bind _returnvalue (Utilities|GetDataTableRow "/Game/MyContent/DataTables/DT_WeaponSettings.DT_WeaponSettings" "Rifle")
    (:then
      (bind _output_get (Variables|Default|SetMaxAmmo (.MaxAmmo (Utilities|Struct|BreakSTRUCT_WeaponSetting _returnvalue))))
      (Variables|Default|SetCurrAmmo _output_get)
      (Variables|Default|SetFireRate (.FireRate (Utilities|Struct|BreakSTRUCT_WeaponSetting _returnvalue))))))

(event Collision|EventActorBeginOverlap
  (params (OtherActor :type Actor%20Object%20Reference))
  (|CallParentFunction OtherActor) ; This node is disabled and will not be called.\nDrag off pins to build functionality.
)

(event EventTick
  (params (DeltaSeconds :type Float%20%28single-precision%29))
  (|CallParentFunction DeltaSeconds) ; This node is disabled and will not be called.\nDrag off pins to build functionality.
)

(fn ConstructionScript
  (|CallParentFunction))