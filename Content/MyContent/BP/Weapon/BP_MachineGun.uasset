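; Machine gun weapon Blueprint that loads its setup from data tables and fires hitscan shots.
; BeginPlay passes the MachineGun row of DT_WeaponSettings to SetWeaponSettings, and GetInfo returns the matching Info from DT_WeaponItemsInfo.
; Shot runs a debug-drawn line trace on the Camera channel and applies Damage through the hit actor's ACBP_Health component, if present.
; Unconnected leftover nodes for random-row printing and weapon spawning never run.
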(event EventBeginPlay
  (|CallParentFunction)
  (bind _returnvalue (Utilities|GetDataTableRow "/Game/MyContent/DataTables/DT_WeaponSettings.DT_WeaponSettings" "MachineGun")
    (:then
      (CallFunction|SetWeaponSettings _returnvalue))))

(event Collision|EventActorBeginOverlap
  (params (OtherActor :type Actor%20Object%20Reference))
  (|CallParentFunction OtherActor) ; This node is disabled and will not be called.\nDrag off pins to build functionality.
)

(event EventTick
  (params (DeltaSeconds :type Float%20%28single-precision%29))
  (|CallParentFunction DeltaSeconds) ; This node is disabled and will not be called.\nDrag off pins to build functionality.
)

(fn ConstructionScript
  (|CallParentFunction))

(fn Shot
  (params (Start :type Vector :default "0, 0, 0") (End :type Vector :default "0, 0, 0"))
  (bind (_outhit _returnvalue) (Collision|LineTraceByChannel Start End "TraceTypeQuery2" false 0 "ForDuration" true "(R=0.010506,G=0.000177,B=0.119792,A=1.000000)" "(R=0.286458,G=0.000000,B=0.002409,A=1.000000)"))
  (if _returnvalue
    ;[0.15 0.15 0.15 0.5] через компонент
    (Utilities|IsValid (Actor|GetComponentbyClass (.HitActor (Collision|BreakHitResult _outhit)) "/Game/MyContent/BP/Weapon/ACBP_Health.ACBP_Health_C")
      (:Is%20Valid
        (Default|Damage (Actor|GetComponentbyClass (.HitActor (Collision|BreakHitResult _outhit)) "/Game/MyContent/BP/Weapon/ACBP_Health.ACBP_Health_C") (Variables|Default|GetDamage))))))

(fn GetInfo
  (bind _returnvalue (Utilities|GetDataTableRow "/Game/MyContent/DataTables/DT_WeaponItemsInfo.DT_WeaponItemsInfo" "MachineGun")
    (:then
      (return (.Info (Utilities|Struct|BreakSTRUCT_WeaponItem _returnvalue))))))