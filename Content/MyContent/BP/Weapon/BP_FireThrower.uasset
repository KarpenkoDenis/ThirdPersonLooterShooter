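; BP_FireThrower is a flamethrower weapon that damages actors overlapping its capsule area.
; BeginPlay loads its DT_WeaponSettings row, then sizes and offsets DamageArea by Range with collision off.
; Shot shows three fire effects, enables collision and starts a MaxAmmo-second timer to StopFire, which hides the effects but leaves collision enabled.
; Overlaps apply damage with a velocity-based impulse through ACBP_Health, also hiding the effects.
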(event OnComponentBeginOverlap(DamageArea)
  (params (OverlappedComponent :type Primitive%20Component%20Object%20Reference) (OtherActor :type Actor%20Object%20Reference) (OtherComp :type Primitive%20Component%20Object%20Reference) (OtherBodyIndex :type Integer) (bFromSweep :type Boolean) (SweepResult :type Hit%20Result%20Structure%20%28by%20ref%29))
  (bind _returnvalue (Actor|GetComponentbyClass OtherActor "/Game/MyContent/BP/Weapon/ACBP_Health.ACBP_Health_C"))
  (if true
    (Utilities|IsValid _returnvalue
      (:Is%20Valid
        (Default|DamagewithImpuls _returnvalue (Variables|Default|GetDamage) (* (Transformation|GetVelocity) 1e+02) (.BoneName (Collision|BreakHitResult SweepResult)))
        (Rendering|SetVisibility (Variables|Default|GetNS_Fire_Big1) false false)))))

(event EventBeginPlay
  (bind _range (Variables|Default|GetRange))
  (bind _damagearea (Variables|Default|GetDamageArea))
  (bind _relativelocation (Variables|/Script/Engine.SceneComponent|GetRelativeLocation _damagearea))
  (|CallParentFunction)
  (bind _returnvalue (Utilities|GetDataTableRow "/Game/MyContent/DataTables/DT_WeaponSettings.DT_WeaponSettings" "FireThrower")
    (:then
      (CallFunction|SetWeaponSettings _returnvalue)
      (Development|PrintString (Utilities|String|ToString(Float) 0.0))
      (Components|Capsule|SetCapsuleHalfHeight _damagearea _range true)
      (Transformation|SetRelativeLocation _damagearea (Math|Vector|MakeVector (.x _relativelocation) (+ (.y _relativelocation) _range) (.z _relativelocation)) false false)
      (Collision|SetCollisionEnabled (Variables|Default|GetDamageArea) "NoCollision"))))

(event Collision|EventActorBeginOverlap
  (params (OtherActor :type Actor%20Object%20Reference))
  (|CallParentFunction OtherActor) ; This node is disabled and will not be called.\nDrag off pins to build functionality.
)

(fn ConstructionScript
  (|CallParentFunction))

(fn Shot
  (params (Start :type Vector :default "0, 0, 0") (End :type Vector :default "0, 0, 0"))
  (Utilities|FlowControl|Sequence
    (:then_0
      (Rendering|SetVisibility (Variables|Default|GetNS_Fire_Big1) true false))
    (:then_1
      (Collision|SetCollisionEnabled (Variables|Default|GetDamageArea) "QueryAndPhysics")
      (Utilities|Time|SetTimerbyFunctionName 0 "StopFire" (Math|Conversions|ToFloat(Integer) (Variables|Default|GetMaxAmmo))))))

(fn StopFire
  (Rendering|SetVisibility (Variables|Default|GetNS_Fire_Big1) false false)
  (Collision|SetCollisionEnabled (Variables|Default|GetDamageArea) "QueryAndPhysics"))